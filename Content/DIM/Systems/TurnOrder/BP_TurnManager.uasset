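; Turn manager that cycles player and enemy characters through a round-robin turn order, with all players ahead of all enemies.
; BeginPlay waits a tick, adds the input mapping, stores the game state and builds the character array.
; NextCharacter clears player movement and menu actors, updates selection, resets the active character's stats, then spawns a player action menu or enemy movement actor.
; IA_EndTurn advances only during a player's turn.
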(event Input|EnhancedActionEvents|EnhancedInputActionIA_EndTurn
  (params (ActionValue :type Boolean) (ElapsedSeconds :type Float%20%28single-precision%29) (TriggeredSeconds :type Float%20%28single-precision%29))
  (Utilities|Casting|CastToBP_PlayerCharacter (CallFunction|CurrentCharacter)) ; Make sure it's a players turn.
  (CallFunction|NextCharacter))

(event EventBeginPlay
  (Utilities|FlowControl|Delay 0.0)
  (Input|AddMappingContext (PlayerController|LocalPlayerSubsystems|GetEnhancedInputLocalPlayerSubsystem (Game|GetPlayerController 0)) "/Game/DIM/Base/Input/IMC_Default.IMC_Default" 0)
  (bind _asgs_base (Utilities|Casting|CastToGS_Base (Game|GetGameState)))
  (Variables|Default|SetGameState _asgs_base)
  ;[0 0 0] Set the character array to be the order of the turns.
  (bind _outactors (Actor|GetAllActorsOfClass "/Game/DIM/Placeables/Characters/BP_PlayerCharacter.BP_PlayerCharacter_C"))
  (Utilities|Array|AppendArray (Variables|Default|GetCharacters) _outactors)
  (bind _outactors_2 (Actor|GetAllActorsOfClass "/Game/DIM/Placeables/Characters/BP_EnemyCharacter.BP_EnemyCharacter_C"))
  (Utilities|Array|AppendArray (Variables|Default|GetCharacters) _outactors_2)
  ;[0 0 0] This will add one at NextCharacter(), so let's just set it to the last index so that it gets mod'd to zero on the first turn.
  (Variables|Default|SetCurrentCharacterIndex (Utilities|Array|LastIndex (Variables|Default|GetCharacters)))
  (CallFunction|NextCharacter))

(fn ConstructionScript)

(fn CurrentCharacter
  (return (Utilities|Array|Get(acopy) (Variables|Default|GetCharacters) (Variables|Default|GetCurrentCharacterIndex))))

(fn NextCharacter
  (bind _character (CallFunction|CurrentCharacter))
  (CallFunction|RemoveExistingInputActors)
  (Variables|Default|SetCurrentCharacterIndex (Math|Integer|%(Integer) (+ (Variables|Default|GetCurrentCharacterIndex) 1) (Utilities|Array|Length (Variables|Default|GetCharacters))))
  ;[0 0 0] Set the selections icon.
  (for _array_element (Variables|Default|GetCharacters)
    (Default|SetIsSelected _array_element (== _array_element (CallFunction|CurrentCharacter))))
  (Default|ResetStats _character)
  (Utilities|Casting|CastToBP_PlayerCharacter _character
    (:then
      (Game|SpawnActorfromClass "/Game/DIM/Systems/PlayerActions/BP_PlayerActionMenu.BP_PlayerActionMenu_C" (Math|Transform|MakeTransform "0, 0, 0" "0, 0, 0" "1,1,1") "Undefined" 0 0))
    (:CastFailed
      (Utilities|Casting|CastToBP_EnemyCharacter _character)
      (Game|SpawnActorfromClass "/Game/DIM/Systems/EnemyActions/BP_EnemyMovement.BP_EnemyMovement_C" (Math|Transform|MakeTransform "0, 0, 0" "0, 0, 0" "1,1,1") "Undefined" 0 0))))

(fn RemoveExistingInputActors
  (Utilities|FlowControl|Sequence
    (:then_0
      (CallFunction|RemovePlayerMovement))
    (:then_1
      (CallFunction|RemoveActionMenu))))