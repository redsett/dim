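; BP_EnemyMovement is a short-lived enemy action actor that walks the current enemy toward the closest player character during its turn.
; On BeginPlay it caches the current enemy and its nearest player target, then waits a random delay for feel before enabling tick.
; Tick moves the enemy toward the target until it is close or can't move, then passes to the next character and destroys itself.
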(event EventBeginPlay
  (bind _character (CallFunction|GetCurrentCharacter))
  (bind _asbp_enemy_character (Utilities|Casting|CastToBP_EnemyCharacter _character))
  (Variables|Default|SetCurrentCharacter _asbp_enemy_character)
  (bind _character_2 (CallFunction|GetClosestPlayerCharacter (Variables|Default|GetCurrentCharacter)))
  (Variables|Default|SetTarget _character_2)
  (Utilities|FlowControl|Delay (Math|Random|RandomFloatinRange 0.5 2.0)) ; Just a feel thing.
  (Actor|Tick|SetActorTickEnabled true))

(event EventTick
  (params (DeltaSeconds :type Float%20%28single-precision%29))
  (bind _target (Variables|Default|GetTarget))
  (bind _currentcharacter (Variables|Default|GetCurrentCharacter))
  (bind _returnvalue (Transformation|GetActorLocation _currentcharacter))
  (bind _returnvalue_2 (Transformation|GetActorLocation _target))
  (CallFunction|MoveCharacter (Variables|Default|GetCurrentCharacter) (Math|Rotator|GetRotationXVector (Math|Rotator|FindLookatRotation _returnvalue _returnvalue_2)) 1.0)
  (if (or (< (Math|Vector|Distance(Vector) _returnvalue _returnvalue_2) 1e+02) (not (Default|CanMove (Variables|Default|GetCurrentCharacter)))) ; Stop moving?
    ;[1 0 0] TODO: Should try to do an action instead of ending the turn.
    (CallFunction|NextCharacter)
    (Actor|DestroyActor)))

(fn ConstructionScript)