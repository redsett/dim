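; BP_PlayerMovement is a player action that lets the player move the current character using Enhanced Input.
; On BeginPlay it removes other instances of its class, adds the movement mapping context and caches the current character.
; Forward and right input move that character along the camera's yaw-only axes, keeping movement on the horizontal plane.
; RemoveSelf removes the mapping context before deferring to the parent's removal logic.
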(event Input|EnhancedActionEvents|EnhancedInputActionIA_MoveForward
  (params (ActionValue :type Float%20%28single-precision%29) (ElapsedSeconds :type Float%20%28single-precision%29) (TriggeredSeconds :type Float%20%28single-precision%29))
  (CallFunction|MoveCharacter (Variables|Default|GetCurrentCharacter) (Math|Vector|GetForwardVector (Math|Rotator|MakeRotator 0.0 0.0 (.Yaw (Math|Rotator|BreakRotator (Camera|GetCameraRotation (Game|GetPlayerCameraManager 0)))))) ActionValue))

(event Input|EnhancedActionEvents|EnhancedInputActionIA_MoveRight
  (params (ActionValue :type Float%20%28single-precision%29) (ElapsedSeconds :type Float%20%28single-precision%29) (TriggeredSeconds :type Float%20%28single-precision%29))
  (CallFunction|MoveCharacter (Variables|Default|GetCurrentCharacter) (Math|Vector|GetRightVector (Math|Rotator|MakeRotator 0.0 0.0 (.Yaw (Math|Rotator|BreakRotator (Camera|GetCameraRotation (Game|GetPlayerCameraManager 0)))))) ActionValue))

(event EventBeginPlay
  (CallFunction|RemoveOthers)
  (Input|AddMappingContext (PlayerController|LocalPlayerSubsystems|GetEnhancedInputLocalPlayerSubsystem (Game|GetPlayerController 0)) "/Game/DIM/Base/Input/Movement/IMC_Movement.IMC_Movement" 0)
  (bind _character (CallFunction|GetCurrentCharacter))
  (Variables|Default|SetCurrentCharacter _character))

(fn ConstructionScript)

(fn RemoveOthers
  (bind _outactors (Actor|GetAllActorsOfClass (Utilities|GetClass self)))
  (for _array_element _outactors
    (if (!= _array_element self)
      (CallFunction|RemoveSelf _array_element))))

(fn RemoveSelf
  (Input|RemoveMappingContext (PlayerController|LocalPlayerSubsystems|GetEnhancedInputLocalPlayerSubsystem (Game|GetPlayerController 0)) "/Game/DIM/Base/Input/Movement/IMC_Movement.IMC_Movement")
  (|CallParentFunction))