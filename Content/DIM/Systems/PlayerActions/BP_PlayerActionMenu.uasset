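; Player action menu actor that maps the four gamepad face buttons to a contextual on-screen menu.
; On BeginPlay it adds its input mapping context, caches the action menu and opens the root menu, forwarding face-button presses to it.
; Each menu function re-initializes labels and delegates; submenus currently show only Back, while the root also spawns BP_PlayerMovement.
; RemoveSelf removes the context, resets the menu and destroys the actor.
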(event Custom|Dummy)

(event Input|EnhancedActionEvents|EnhancedInputActionIA_ActionMenuFaceBottom
  (params (ActionValue :type Boolean) (ElapsedSeconds :type Float%20%28single-precision%29) (TriggeredSeconds :type Float%20%28single-precision%29))
  (Default|Pressed (Variables|Default|GetActionMenuRef) "NewEnumerator5"))

(event Input|EnhancedActionEvents|EnhancedInputActionIA_ActionMenuFaceTop
  (params (ActionValue :type Boolean) (ElapsedSeconds :type Float%20%28single-precision%29) (TriggeredSeconds :type Float%20%28single-precision%29))
  (Default|Pressed (Variables|Default|GetActionMenuRef) "NewEnumerator4"))

(event Input|EnhancedActionEvents|EnhancedInputActionIA_ActionMenuFaceRight
  (params (ActionValue :type Boolean) (ElapsedSeconds :type Float%20%28single-precision%29) (TriggeredSeconds :type Float%20%28single-precision%29))
  (Default|Pressed (Variables|Default|GetActionMenuRef) "NewEnumerator6"))

(event Input|EnhancedActionEvents|EnhancedInputActionIA_ActionMenuFaceLeft
  (params (ActionValue :type Boolean) (ElapsedSeconds :type Float%20%28single-precision%29) (TriggeredSeconds :type Float%20%28single-precision%29))
  (Default|Pressed (Variables|Default|GetActionMenuRef) "NewEnumerator7"))

(event EventBeginPlay
  (Input|AddMappingContext (PlayerController|LocalPlayerSubsystems|GetEnhancedInputLocalPlayerSubsystem (Game|GetPlayerController 0)) "/Game/DIM/Base/Input/ActionMenu/IMC_ActionMenu.IMC_ActionMenu" 0)
  (bind _actionmenu (CallFunction|GetActionMenu))
  (Variables|Default|SetActionMenuRef _actionmenu)
  (CallFunction|RootMenu))

(fn ConstructionScript)

(fn RemoveSelf
  (Input|RemoveMappingContext (PlayerController|LocalPlayerSubsystems|GetEnhancedInputLocalPlayerSubsystem (Game|GetPlayerController 0)) "/Game/DIM/Base/Input/ActionMenu/IMC_ActionMenu.IMC_ActionMenu")
  (Default|Init :self (Variables|Default|GetActionMenuRef) :TopEvent (EventDispatchers|CreateEvent :!event Custom|Dummy) :BottomEvent (EventDispatchers|CreateEvent :!event Custom|Dummy) :RightEvent (EventDispatchers|CreateEvent :!event Custom|Dummy) :LeftEvent (EventDispatchers|CreateEvent :!event Custom|Dummy))
  (Actor|DestroyActor))

(fn BasicAttack
  (Default|Init :self (Variables|Default|GetActionMenuRef) :Right (Utilities|Struct|MakeS_ActionMenuWidget true false "Back") :TopEvent (EventDispatchers|CreateEvent :!event Custom|Dummy) :BottomEvent (EventDispatchers|CreateEvent :!event Custom|Dummy) :RightEvent (EventDispatchers|CreateEvent :!event RootMenu) :LeftEvent (EventDispatchers|CreateEvent :!event Custom|Dummy)))

(fn Abilities
  (Default|Init :self (Variables|Default|GetActionMenuRef) :Right (Utilities|Struct|MakeS_ActionMenuWidget true false "Back") :TopEvent (EventDispatchers|CreateEvent :!event Custom|Dummy) :BottomEvent (EventDispatchers|CreateEvent :!event Custom|Dummy) :RightEvent (EventDispatchers|CreateEvent :!event RootMenu) :LeftEvent (EventDispatchers|CreateEvent :!event Custom|Dummy)))

(fn Equipment
  (Default|Init :self (Variables|Default|GetActionMenuRef) :Right (Utilities|Struct|MakeS_ActionMenuWidget true false "Back") :TopEvent (EventDispatchers|CreateEvent :!event Custom|Dummy) :BottomEvent (EventDispatchers|CreateEvent :!event Custom|Dummy) :RightEvent (EventDispatchers|CreateEvent :!event RootMenu) :LeftEvent (EventDispatchers|CreateEvent :!event Custom|Dummy)))

(fn RootMenu
  (Default|Init :self (Variables|Default|GetActionMenuRef) :Top (Utilities|Struct|MakeS_ActionMenuWidget true false "Equipment") :Bottom (Utilities|Struct|MakeS_ActionMenuWidget true false "Basic Attack") :Left (Utilities|Struct|MakeS_ActionMenuWidget true false "Abilities") :TopEvent (EventDispatchers|CreateEvent :!event Equipment) :BottomEvent (EventDispatchers|CreateEvent :!event BasicAttack) :RightEvent (EventDispatchers|CreateEvent :!event Custom|Dummy) :LeftEvent (EventDispatchers|CreateEvent :!event Abilities))
  (Game|SpawnActorfromClass "/Game/DIM/Systems/PlayerActions/BP_PlayerMovement.BP_PlayerMovement_C" (Math|Transform|MakeTransform "0, 0, 0" "0, 0, 0" "1,1,1") "Undefined" 0 0))