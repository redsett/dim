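; BP_Character is a base character with limited movement distance and basic attacks, plus a selection indicator.
; ResetStats refills both budgets, MoveCharacter subtracts moved distance with a floor of zero, and DoBasicAttack spends one attack and reports success.
; CanMove and CanBasicAttack gate those actions, while SetIsSelected toggles the selection mesh.
; The construction script makes the extra skeletal mesh follow the main Mesh through master pose.
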(fn ConstructionScript
  (Class|SkinnedMeshComponent|SetMasterPoseComponent (Variables|Default|GetSkeletalMesh) (Variables|Character|GetMesh) false))

(fn ResetStats
  (Variables|CurrentStats|SetCurrentMoveDistance (Variables|BaseStats|GetMoveDistance))
  (Variables|CurrentStats|SetCurrentBasicAttacksRemaining (Variables|BaseStats|GetBasicAttacksRemaining)))

(fn MoveCharacter
  (params (MovedAmount :type Float%20%28single-precision%29))
  (if (Movement|CanMove)
    (bind _output_get (Variables|CurrentStats|SetCurrentMoveDistance (|(max((v-amount),0)) (stale _output_get) MovedAmount)))))

(fn CanMove
  (return (> (Variables|CurrentStats|GetCurrentMoveDistance) 0.0)))

(fn SetIsSelected
  (params (Selected :type Boolean))
  (Rendering|SetVisibility (Variables|Default|GetSelectionVisualMesh) Selected false))

(fn DoBasicAttack
  (if (BasicAttack|CanBasicAttack)
    (Math|Integer|DecrementInt (Variables|CurrentStats|GetCurrentBasicAttacksRemaining)
      (:%20%20
        (return true)))
    (else
      (return false))))

(fn CanBasicAttack
  (return (> (Variables|CurrentStats|GetCurrentBasicAttacksRemaining) 0)))