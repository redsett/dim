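; A VFX Blueprint that moves a particle system along a spline path to form a trail effect.
; On BeginPlay, the Duralation variable sets the timeline's play rate, and the timeline starts from a random time so its starting point varies.
; Each update maps the timeline alpha to a distance along the spline, placing the particles there in world space at a fixed half scale.
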(event EventBeginPlay
  (bind _spline (Variables|Default|GetSpline))
  (bind _particlesystem (Variables|Default|GetParticleSystem))
  (Components|Timeline|SetPlayRate (Variables|Default|GetTimeline_0) (Variables|Default|GetDuralation))
  (Utilities|FlowControl|Sequence
    (:then_0
      (bind _alpha (Timeline|Timeline_0 SetNewTime)
        (:Update
          (Transformation|SetWorldLocation _particlesystem (Spline|GetLocationatDistanceAlongSpline _spline (* (Spline|GetSplineLength _spline) _alpha) "World") false false)
          (Transformation|SetWorldScale3D _particlesystem "0.500000,0.500000,0.500000"))))
    (:then_1
      (Timeline|Timeline_0 Play))))

(fn ConstructionScript)